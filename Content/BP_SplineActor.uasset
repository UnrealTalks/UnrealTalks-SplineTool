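; Spline actor that builds a railing in the construction script, with optional fence posts and street lights.
; GetMeshLength rounds spline length over an ideal length to get equal segments; its min/max correction loop never runs.
; Each segment gets a spline mesh with length-scaled tangents.
; Posts are instanced at segment boundaries except the start, lights at midpoints, each with a downward spot light component.
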(fn `AddFencePost`
  (params (Index :type Integer))
  (bind _spline (`self.Spline`))
  (bind _returnvalue (* Index (`self.MeshLength`)))
  (bind (_returnvalue_roll _returnvalue_pitch _returnvalue_yaw) (`KismetMathLibrary.BreakRotator` (`KismetMathLibrary.MakeRotFromX` (`SplineComponent.GetTangentAtDistanceAlongSpline` _spline _returnvalue "Local"))))
  (`InstancedStaticMeshComponent.AddInstance` (`self.FencePost`) (`KismetMathLibrary.MakeTransform` (`SplineComponent.GetLocationAtDistanceAlongSpline` _spline _returnvalue "Local") (`KismetMathLibrary.MakeRotator` 0.0 0.0 _returnvalue_yaw))))

(fn `AddStreeLight`
  (params (Index :type Integer))
  (bind _meshlength (`self.MeshLength`))
  (bind _spline (`self.Spline`))
  (bind _returnvalue (+ (* Index _meshlength) (/ _meshlength 2.0)))
  (bind _returnvalue_2 (`SplineComponent.GetLocationAtDistanceAlongSpline` _spline _returnvalue "Local"))
  (bind (_returnvalue_roll _returnvalue_pitch _returnvalue_yaw) (`KismetMathLibrary.BreakRotator` (`KismetMathLibrary.MakeRotFromX` (`SplineComponent.GetTangentAtDistanceAlongSpline` _spline _returnvalue "Local"))))
  (`InstancedStaticMeshComponent.AddInstance` (`self.StreetLight`) (`KismetMathLibrary.MakeTransform` _returnvalue_2 (`KismetMathLibrary.MakeRotator` 0.0 0.0 _returnvalue_yaw)))
  (`AddComponent|NODE_AddSpotLightComponent-1` :`RelativeTransform` (`KismetMathLibrary.MakeTransform` (+ _returnvalue_2 (0.0 0.0 200.0)) (`KismetMathLibrary.MakeRotator` 0.0 -90.0))))

(fn `FindStartAndEnd`
  (params (Index :type Integer))
  (returns (ReturnValue :type "Vector Structure") (ReturnValue3 :type "Vector Structure") (ReturnValue2 :type "Vector Structure") (ReturnValue4 :type "Vector Structure"))
  (bind _spline (`self.Spline`))
  (bind _meshlength (`self.MeshLength`))
  (bind _meshlength_2 (`self.MeshLength`))
  (bind _spline_2 (`self.Spline`))
  (bind _returnvalue (* (+ Index 1) _meshlength))
  (bind _returnvalue_2 (* Index _meshlength))
  (return (`SplineComponent.GetLocationAtDistanceAlongSpline` _spline _returnvalue_2 "Local") (* (`KismetMathLibrary.Normal` (`SplineComponent.GetTangentAtDistanceAlongSpline` _spline _returnvalue_2 "Local")) _meshlength_2) (`SplineComponent.GetLocationAtDistanceAlongSpline` _spline_2 _returnvalue "Local") (* (`KismetMathLibrary.Normal` (`SplineComponent.GetTangentAtDistanceAlongSpline` _spline_2 _returnvalue "Local")) _meshlength_2)))

(fn `GetMeshLength`
  (bind _returnvalue (`SplineComponent.GetSplineLength` (`self.Spline`)))
  (bind _returnvalue_2 (`KismetMathLibrary.Round` (/ _returnvalue (`self.MeshLengthIdeal`))))
  (set `self.Divisions` _returnvalue_2)
  (set `self.MeshLength` (/ _returnvalue (`KismetMathLibrary.Conv_IntToDouble` _returnvalue_2))))

(fn `UserConstructionScript`
  (bind _divisions (`self.Divisions`))
  (`SplineComponent.SetClosedLoop` (`self.Spline`) (`self.Closed Loop?`) true)
  (`self.GetMeshLength`)
  (for _index (range (+ _divisions 1))
    (`|ExecutionSequence`
      (:`then_0`
        (if (and (`self.AddFencePost?`) (!= _index 0))
          (`self.AddFencePost` _index)))
      (:`then_1`
        (bind _returnvalue (!= _index _divisions))
        (if _returnvalue
          (bind _returnvalue_2 (`AddComponent|NODE_AddSplineMeshComponent-0`))
          (bind (_returnvalue_3 _returnvalue3 _returnvalue2 _returnvalue4) (`self.FindStartAndEnd` _index))
          (`SplineMeshComponent.SetStartAndEnd` _returnvalue_2 _returnvalue_3 _returnvalue3 _returnvalue2 _returnvalue4 true)
          (`StaticMeshComponent.SetStaticMesh` _returnvalue_2 (`self.RailMesh`))))
      (:`then_2`
        (if (and _returnvalue (`self.AddStreetLight?`))
          (`self.AddStreeLight` _index))))))